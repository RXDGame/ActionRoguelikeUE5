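; Bonfire Blueprint that acts as an interactable save point, offering "Save Game" as its interact text.
; Interact sets FireEnabled, writes the save game through SGameModeBase, prints a confirmation and calls UpdateFire to activate the particle effect.
; OnActorLoaded also calls UpdateFire, so the fire activates on load if FireEnabled is set.
; CanInteract always returns false as written.
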(event Custom|UpdateFire
  (if (Variables|Default|GetbFireEnabled)
    (Components|Activation|Activate (Variables|Default|GetParticleSystem) false)))

(event EventOnActorLoaded
  (CallFunction|UpdateFire))

(event EventInteract
  (params (InstigatorPawn :type Pawn%20Object%20Reference))
  (Variables|Default|SetbFireEnabled true)
  (bind _assgame_mode_base (Utilities|Casting|CastToSGameModeBase (Game|GetGameMode)))
  (Class|SGameModeBase|WriteSaveGame _assgame_mode_base)
  (Development|PrintString "WORLD SAVED")
  (CallFunction|UpdateFire))

(fn ConstructionScript)

(fn CanInteract
  (params (InstigatorPawn :type Pawn%20Object%20Reference))
  (return false))

(fn GetInteractText
  (params (InstigatorPawn :type Pawn%20Object%20Reference))
  (return "Save Game"))